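; Scene capture actor that saves snapshots of its 2D scene capture view as timestamped JPG files.
; BeginPlay creates an RGBA8 render target at the configured size and binds it to the capture component.
; The Capture event renders the scene, exports the texture to a hard-coded C:/tmp folder and prints the result on completion.
; FilenameFromTime builds the name from unpadded date and time parts, duplicating the unused TimeToString helper.
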(event `self.ReceiveBeginPlay`
  (bind _returnvalue (`KismetRenderingLibrary.CreateRenderTarget2D` (`self.Width`) (`self.Height`) "RTF_RGBA8"))
  (bind _output_get (set `self.TargetTexture` _returnvalue))
  (set `SceneCaptureComponent2D.TextureTarget` _output_get (`self.SceneCaptureComponent2D`)))

(event `Capture`
  (bind _scenecapturecomponent2d (`self.SceneCaptureComponent2D`))
  (`SceneCaptureComponent2D.CaptureScene` _scenecapturecomponent2d)
  (bind _filename (`self.FilenameFromTime` "C:/tmp/" "Capture2D_" "" ".jpg"))
  (`ImageWriteBlueprintLibrary.ExportToDisk` (`SceneCaptureComponent2D.TextureTarget` _scenecapturecomponent2d) _filename (make `ImageWriteOptions` "JPG" (delegate `OnCompleteExport`))))

(event `OnCompleteExport`
  (params (bSuccess :type Boolean))
  (`KismetSystemLibrary.PrintString` (`KismetStringLibrary.Concat_StrStr` "Capture Saved: [" (`KismetStringLibrary.Conv_BoolToString` bSuccess) "] " (stale `Capture` _filename))))

(fn `FilenameFromTime`
  (params (OutputFolder :type String) (Prefix :type String) (PostFix :type String) (Extension :type String))
  (returns (Filename :type String))
  (bind (_returnvalue_year _returnvalue_month _returnvalue_day _returnvalue_hour _returnvalue_minute _returnvalue_second) (`KismetMathLibrary.BreakDateTime` (`KismetMathLibrary.Now`)))
  (return (`KismetStringLibrary.Concat_StrStr` OutputFolder Prefix (`KismetStringLibrary.Concat_StrStr` (`KismetStringLibrary.Conv_IntToString` _returnvalue_year) (`KismetStringLibrary.Conv_IntToString` _returnvalue_month) (`KismetStringLibrary.Conv_IntToString` _returnvalue_day) "_" (`KismetStringLibrary.Conv_IntToString` _returnvalue_hour) (`KismetStringLibrary.Conv_IntToString` _returnvalue_minute) (`KismetStringLibrary.Conv_IntToString` _returnvalue_second)) PostFix Extension)))

(fn `TimeToString`
  (returns (Time :type String))
  (bind (_returnvalue_year _returnvalue_month _returnvalue_day _returnvalue_hour _returnvalue_minute _returnvalue_second) (`KismetMathLibrary.BreakDateTime` (`KismetMathLibrary.Now`)))
  (return (`KismetStringLibrary.Concat_StrStr` (`KismetStringLibrary.Conv_IntToString` _returnvalue_year) (`KismetStringLibrary.Conv_IntToString` _returnvalue_month) (`KismetStringLibrary.Conv_IntToString` _returnvalue_day) "_" (`KismetStringLibrary.Conv_IntToString` _returnvalue_hour) (`KismetStringLibrary.Conv_IntToString` _returnvalue_minute) (`KismetStringLibrary.Conv_IntToString` _returnvalue_second))))

(fn `UserConstructionScript`)