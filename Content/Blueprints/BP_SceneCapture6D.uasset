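; Six-direction scene capture actor that saves N, S, E, W, up and down views of the level as JPG files.
; The construction script gives each of six SceneCapture2D components its own RGBA8 render target sized by Width and Height.
; SaveScene captures all six, exports them with a shared game-time filename plus direction suffix, and prints each result.
; A separate Capture event saves only the north view to a hardcoded folder, named by wall-clock date and time.
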(event `Capture`
  (bind _scenecapturecomponent2d_n (`self.SceneCaptureComponent2D_N`))
  (`SceneCaptureComponent2D.CaptureScene` _scenecapturecomponent2d_n)
  (bind _filename (`self.FilenameFromTime` "C:/tmp/" "Capture2D_" "" ".jpg"))
  (`ImageWriteBlueprintLibrary.ExportToDisk` (`SceneCaptureComponent2D.TextureTarget` _scenecapturecomponent2d_n) _filename (make `ImageWriteOptions` "JPG" (delegate `OnCompleteExport`))))

(event `OnCompleteExport`
  (params (bSuccess :type Boolean))
  (`KismetSystemLibrary.PrintString` (`KismetStringLibrary.Concat_StrStr` "Capture Saved: [" (`KismetStringLibrary.Conv_BoolToString` bSuccess) "] " (stale `Capture` _filename))))

(event `OnImageSaved_N`
  (params (bSuccess :type Boolean))
  (`KismetSystemLibrary.PrintString` (`KismetStringLibrary.Concat_StrStr` "Capture Saved: [" (`KismetStringLibrary.Conv_BoolToString` bSuccess) "] " (`KismetStringLibrary.Concat_StrStr` (`self.FileName`) (`self.TimeSecondsStr`) "_N.jpg"))))

(event `OnImageSaved_S`
  (params (bSuccess :type Boolean))
  (`KismetSystemLibrary.PrintString` (`KismetStringLibrary.Concat_StrStr` "Capture Saved: [" (`KismetStringLibrary.Conv_BoolToString` bSuccess) "] " (`KismetStringLibrary.Concat_StrStr` (`self.FileName`) (`self.TimeSecondsStr`) "_S.jpg"))))

(event `SaveScene`
  (`self.CaptureScene`)
  (set `self.FileName` (`KismetStringLibrary.Concat_StrStr` (`self.OutputDir`) (`self.FileNamePrefix`) "_"))
  (set `self.TimeSecondsStr` (`KismetStringLibrary.Conv_DoubleToString` (`GameplayStatics.GetTimeSeconds`)))
  (`|ExecutionSequence`
    (:`then_0`
      (`ImageWriteBlueprintLibrary.ExportToDisk` (`SceneCaptureComponent2D.TextureTarget` (`self.SceneCaptureComponent2D_N`)) (`KismetStringLibrary.Concat_StrStr` (`self.FileName`) (`self.TimeSecondsStr`) "_N.jpg") (make `ImageWriteOptions` "JPG" (delegate `OnImageSaved_N`))))
    (:`then_1`
      (`ImageWriteBlueprintLibrary.ExportToDisk` (`SceneCaptureComponent2D.TextureTarget` (`self.SceneCaptureComponent2D_S`)) (`KismetStringLibrary.Concat_StrStr` (`self.FileName`) (`self.TimeSecondsStr`) "_S.jpg") (make `ImageWriteOptions` "JPG" (delegate `OnImageSaved_S`))))
    (:`then_2`
      (`ImageWriteBlueprintLibrary.ExportToDisk` (`SceneCaptureComponent2D.TextureTarget` (`self.SceneCaptureComponent2D_E`)) (`KismetStringLibrary.Concat_StrStr` (`self.FileName`) (`self.TimeSecondsStr`) "_E.jpg") (make `ImageWriteOptions` "JPG" (delegate `OnImageSaved_E`))))
    (:`then_3`
      (`ImageWriteBlueprintLibrary.ExportToDisk` (`SceneCaptureComponent2D.TextureTarget` (`self.SceneCaptureComponent2D_W`)) (`KismetStringLibrary.Concat_StrStr` (`self.FileName`) (`self.TimeSecondsStr`) "_W.jpg") (make `ImageWriteOptions` "JPG" (delegate `OnImageSaved_W`))))
    (:`then_4`
      (`ImageWriteBlueprintLibrary.ExportToDisk` (`SceneCaptureComponent2D.TextureTarget` (`self.SceneCaptureComponent2D_U`)) (`KismetStringLibrary.Concat_StrStr` (`self.FileName`) (`self.TimeSecondsStr`) "_U.jpg") (make `ImageWriteOptions` "JPG" (delegate `OnImageSaved_U`))))
    (:`then_5`
      (`ImageWriteBlueprintLibrary.ExportToDisk` (`SceneCaptureComponent2D.TextureTarget` (`self.SceneCaptureComponent2D_D`)) (`KismetStringLibrary.Concat_StrStr` (`self.FileName`) (`self.TimeSecondsStr`) "_D.jpg") (make `ImageWriteOptions` "JPG" (delegate `OnImageSaved_D`))))))

(event `OnImageSaved_E`
  (params (bSuccess :type Boolean))
  (`KismetSystemLibrary.PrintString` (`KismetStringLibrary.Concat_StrStr` "Capture Saved: [" (`KismetStringLibrary.Conv_BoolToString` bSuccess) "] " (`KismetStringLibrary.Concat_StrStr` (`self.FileName`) (`self.TimeSecondsStr`) "_E.jpg"))))

(event `OnImageSaved_W`
  (params (bSuccess :type Boolean))
  (`KismetSystemLibrary.PrintString` (`KismetStringLibrary.Concat_StrStr` "Capture Saved: [" (`KismetStringLibrary.Conv_BoolToString` bSuccess) "] " (`KismetStringLibrary.Concat_StrStr` (`self.FileName`) (`self.TimeSecondsStr`) "_W.jpg"))))

(event `OnImageSaved_U`
  (params (bSuccess :type Boolean))
  (`KismetSystemLibrary.PrintString` (`KismetStringLibrary.Concat_StrStr` "Capture Saved: [" (`KismetStringLibrary.Conv_BoolToString` bSuccess) "] " (`KismetStringLibrary.Concat_StrStr` (`self.FileName`) (`self.TimeSecondsStr`) "_U.jpg"))))

(event `OnImageSaved_D`
  (params (bSuccess :type Boolean))
  (`KismetSystemLibrary.PrintString` (`KismetStringLibrary.Concat_StrStr` "Capture Saved: [" (`KismetStringLibrary.Conv_BoolToString` bSuccess) "] " (`KismetStringLibrary.Concat_StrStr` (`self.FileName`) (`self.TimeSecondsStr`) "_D.jpg"))))

(fn `CaptureScene`
  (`|ExecutionSequence`
    (:`then_0`
      (`SceneCaptureComponent2D.CaptureScene` (`self.SceneCaptureComponent2D_N`)))
    (:`then_1`
      (`SceneCaptureComponent2D.CaptureScene` (`self.SceneCaptureComponent2D_S`)))
    (:`then_2`
      (`SceneCaptureComponent2D.CaptureScene` (`self.SceneCaptureComponent2D_E`)))
    (:`then_3`
      (`SceneCaptureComponent2D.CaptureScene` (`self.SceneCaptureComponent2D_W`)))
    (:`then_4`
      (`SceneCaptureComponent2D.CaptureScene` (`self.SceneCaptureComponent2D_U`)))
    (:`then_5`
      (`SceneCaptureComponent2D.CaptureScene` (`self.SceneCaptureComponent2D_D`)))))

(fn `FilenameFromTime`
  (params (OutputFolder :type String) (Prefix :type String) (PostFix :type String) (Extension :type String))
  (returns (Filename :type String))
  (bind (_returnvalue_year _returnvalue_month _returnvalue_day _returnvalue_hour _returnvalue_minute _returnvalue_second) (`KismetMathLibrary.BreakDateTime` (`KismetMathLibrary.Now`)))
  (return (`KismetStringLibrary.Concat_StrStr` OutputFolder Prefix (`KismetStringLibrary.Concat_StrStr` (`KismetStringLibrary.Conv_IntToString` _returnvalue_year) (`KismetStringLibrary.Conv_IntToString` _returnvalue_month) (`KismetStringLibrary.Conv_IntToString` _returnvalue_day) "_" (`KismetStringLibrary.Conv_IntToString` _returnvalue_hour) (`KismetStringLibrary.Conv_IntToString` _returnvalue_minute) (`KismetStringLibrary.Conv_IntToString` _returnvalue_second)) PostFix Extension)))

(fn `TimeToString`
  (returns (Time :type String))
  (bind (_returnvalue_year _returnvalue_month _returnvalue_day _returnvalue_hour _returnvalue_minute _returnvalue_second) (`KismetMathLibrary.BreakDateTime` (`KismetMathLibrary.Now`)))
  (return (`KismetStringLibrary.Concat_StrStr` (`KismetStringLibrary.Conv_IntToString` _returnvalue_year) (`KismetStringLibrary.Conv_IntToString` _returnvalue_month) (`KismetStringLibrary.Conv_IntToString` _returnvalue_day) "_" (`KismetStringLibrary.Conv_IntToString` _returnvalue_hour) (`KismetStringLibrary.Conv_IntToString` _returnvalue_minute) (`KismetStringLibrary.Conv_IntToString` _returnvalue_second))))

(fn `UserConstructionScript`
  (`|ExecutionSequence`
    (:`then_0`
      (bind _returnvalue (`KismetRenderingLibrary.CreateRenderTarget2D` (`self.Width`) (`self.Height`) "RTF_RGBA8"))
      (set `SceneCaptureComponent2D.TextureTarget` _returnvalue (`self.SceneCaptureComponent2D_N`)))
    (:`then_1`
      (bind _returnvalue_2 (`KismetRenderingLibrary.CreateRenderTarget2D` (`self.Width`) (`self.Height`) "RTF_RGBA8"))
      (set `SceneCaptureComponent2D.TextureTarget` _returnvalue_2 (`self.SceneCaptureComponent2D_S`)))
    (:`then_2`
      (bind _returnvalue_3 (`KismetRenderingLibrary.CreateRenderTarget2D` (`self.Width`) (`self.Height`) "RTF_RGBA8"))
      (set `SceneCaptureComponent2D.TextureTarget` _returnvalue_3 (`self.SceneCaptureComponent2D_E`)))
    (:`then_3`
      (bind _returnvalue_4 (`KismetRenderingLibrary.CreateRenderTarget2D` (`self.Width`) (`self.Height`) "RTF_RGBA8"))
      (set `SceneCaptureComponent2D.TextureTarget` _returnvalue_4 (`self.SceneCaptureComponent2D_W`)))
    (:`then_4`
      (bind _returnvalue_5 (`KismetRenderingLibrary.CreateRenderTarget2D` (`self.Width`) (`self.Height`) "RTF_RGBA8"))
      (set `SceneCaptureComponent2D.TextureTarget` _returnvalue_5 (`self.SceneCaptureComponent2D_U`)))
    (:`then_5`
      (bind _returnvalue_6 (`KismetRenderingLibrary.CreateRenderTarget2D` (`self.Width`) (`self.Height`) "RTF_RGBA8"))
      (set `SceneCaptureComponent2D.TextureTarget` _returnvalue_6 (`self.SceneCaptureComponent2D_D`)))))