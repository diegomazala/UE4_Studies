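; Scene capture actor that renders a cube map of its surroundings and saves it to disk as an EXR file.
; BeginPlay assigns the target texture to the cube capture component, and the Capture event renders the scene and exports the cube map synchronously.
; FilenameFromTime builds a timestamped path under a hardcoded C:/tmp/ folder, and a completion callback prints the save result.
; Alternative render target export nodes are left unconnected.
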(event `self.ReceiveBeginPlay`
  (set `SceneCaptureComponentCube.TextureTarget` (`self.TargetTexture`) (`self.SceneCaptureComponentCube`)))

(event `Capture`
  (bind _scenecapturecomponentcube (`self.SceneCaptureComponentCube`))
  (`SceneCaptureComponentCube.CaptureScene` _scenecapturecomponentcube)
  (bind _filename (`self.FilenameFromTime` "C:/tmp/" "CaptureCube_" "" ".exr"))
  (`ImageWriteBlueprintLibrary.ExportCubeMapToDisk` (`SceneCaptureComponentCube.TextureTarget` _scenecapturecomponentcube) _filename (make `ImageWriteOptions` "EXR" (delegate `OnCaptureSaved`) 0 true false)))

(event `OnCaptureSaved`
  (params (bSuccess :type Boolean))
  (`KismetSystemLibrary.PrintString` (`KismetStringLibrary.Concat_StrStr` "Capture Saved: [" (`KismetStringLibrary.Conv_BoolToString` bSuccess) "] " (stale `Capture` _filename))))

(fn `FilenameFromTime`
  (params (OutputFolder :type String) (Prefix :type String) (PostFix :type String) (Extension :type String))
  (returns (Filename :type String))
  (bind (_returnvalue_year _returnvalue_month _returnvalue_day _returnvalue_hour _returnvalue_minute _returnvalue_second) (`KismetMathLibrary.BreakDateTime` (`KismetMathLibrary.Now`)))
  (return (`KismetStringLibrary.Concat_StrStr` OutputFolder Prefix (`KismetStringLibrary.Concat_StrStr` (`KismetStringLibrary.Conv_IntToString` _returnvalue_year) (`KismetStringLibrary.Conv_IntToString` _returnvalue_month) (`KismetStringLibrary.Conv_IntToString` _returnvalue_day) "_" (`KismetStringLibrary.Conv_IntToString` _returnvalue_hour) (`KismetStringLibrary.Conv_IntToString` _returnvalue_minute) (`KismetStringLibrary.Conv_IntToString` _returnvalue_second)) PostFix Extension)))

(fn `TimeToString`
  (returns (Time :type String))
  (bind (_returnvalue_year _returnvalue_month _returnvalue_day _returnvalue_hour _returnvalue_minute _returnvalue_second) (`KismetMathLibrary.BreakDateTime` (`KismetMathLibrary.Now`)))
  (return (`KismetStringLibrary.Concat_StrStr` (`KismetStringLibrary.Conv_IntToString` _returnvalue_year) (`KismetStringLibrary.Conv_IntToString` _returnvalue_month) (`KismetStringLibrary.Conv_IntToString` _returnvalue_day) "_" (`KismetStringLibrary.Conv_IntToString` _returnvalue_hour) (`KismetStringLibrary.Conv_IntToString` _returnvalue_minute) (`KismetStringLibrary.Conv_IntToString` _returnvalue_second))))

(fn `UserConstructionScript`)